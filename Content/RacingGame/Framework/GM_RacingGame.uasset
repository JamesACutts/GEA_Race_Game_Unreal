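; Racing game mode that runs the start countdown, lap count and end of race.
; On BeginPlay it binds an event to the checkpoint-hit dispatcher of each finish-line BP_Checkpoint, then starts a timed countdown into GameStart.
; UpdateLaps adds to the lap count, or calls GameEnd once the count equals the lap total.
; Countdown, start, lap and finish stages currently give only debug-print feedback.
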(event Custom|Game%20Start
  (Development|PrintString "Game has started"))

(event Custom|Countdown
  (Development|PrintString "CountDown")
  (Utilities|FlowControl|Delay (Variables|Default|GetCountdownDuration))
  (CallFunction|GameStart))

(event Custom|UpdateLaps
  (params (AddLap :type Integer))
  (if (== (Variables|Default|GetLap) (Variables|Default|GetNumOfLaps))
    (CallFunction|GameEnd)
    (else
      (CallFunction|Laps AddLap)
      (Development|PrintString "Lap Added"))))

(event Custom|Game%20End
  (Development|PrintString "Game Finished"))

(event EventBeginPlay
  (Utilities|FlowControl|Sequence
    (:then_0
      (bind _outactors (Actor|GetAllActorsOfClass "/Game/RacingGame/Checkpoints/BP_Checkpoint.BP_Checkpoint_C"))
      (for _array_element _outactors
        (if (Variables|/Game/RacingGame/Checkpoints/BP_Checkpoint.BP_Checkpoint_C|GetisFinishLine _array_element)
          (EventDispatchers|BindEventtoOnCheckpointHit _array_element (EventDispatchers|CreateEvent :!event Custom|UpdateLaps)))))
    (:then_1
      (CallFunction|Countdown))))

(event EventTick
  (params (DeltaSeconds :type Float%20%28single-precision%29)))

(fn ConstructionScript)

(fn Laps
  (params (AddLap :type Integer))
  (Variables|Default|SetLap (+ (Variables|Default|GetLap) AddLap)))